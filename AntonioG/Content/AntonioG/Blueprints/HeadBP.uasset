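; HeadBP is a player-controlled head that rolls and hops using physics.
; Movement axes apply roll torque, while the Breathe axis applies a scaled forward-and-up velocity impulse when CanJump is set.
; Each Breathe axis update clears CanJump, even at zero input, and any Hit event restores it.
; It also prints "Win" on WinTrigger overlap and toggles the pause menu, game pause and cursor via an Escape FlipFlop.
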(event `InputAxis|MoveForward`
  (params (AxisValue :type "Float (single-precision)"))
  ;[1 0 0.01667 0.686] Move Forward & Backward
  (`PrimitiveComponent.AddTorqueInRadians` (`self.Head`) (`KismetMathLibrary.MakeVector` 0.0 (* (`self.RollTorque`) AxisValue -1.0)) "None" false))

(event `InputAxis|MoveRight`
  (params (AxisValue :type "Float (single-precision)"))
  ;[1 0 0.02469 0.686] Move Left & Right
  (`PrimitiveComponent.AddTorqueInRadians` (`self.Head`) (`KismetMathLibrary.MakeVector` (* (`self.RollTorque`) AxisValue -1.0)) "None" false))

(event `InputAxis|Breathe`
  (params (AxisValue :type "Float (single-precision)"))
  ;[1 0 0 0.686] Airtime
  (if (`self.canJump`)
    (`PrimitiveComponent.AddImpulse` (`self.Head`) (`KismetMathLibrary.MakeVector` (* AxisValue (`self.jumpThrust`)) 0.0 (* AxisValue (`self.jumpHeight`))) "None" true)
    (set `self.canJump` false)))

(event `self.ReceiveHit`
  (params (MyComp :type "PrimitiveComponent Object Reference") (Other :type "Actor Object Reference") (OtherComp :type "PrimitiveComponent Object Reference") (bSelfMoved :type Boolean) (HitLocation :type "Vector Structure") (HitNormal :type "Vector Structure") (NormalImpulse :type "Vector Structure") (Hit :type "HitResult Structure (by ref)"))
  ;[1 0 0 0.686] Airtime
  (set `self.canJump` true))

(event `self.winTrigger.OnActorBeginOverlap`
  (params (OverlappedActor :type "Actor Object Reference") (OtherActor :type "Actor Object Reference"))
  (`KismetSystemLibrary.PrintString` "Win"))

(event `Key|Escape` :paused true
  (params (Key :type "Key Structure"))
  (bind _returnvalue (`GameplayStatics.GetPlayerController` 0))
  (:`Pressed`
    (`/Engine/EditorBlueprintResources/StandardMacros.FlipFlop`
      (:`A`
        (bind _returnvalue_2 (`|CreateWidget` "/Game/AntonioG/Pause_Menu/Pause_MenuWidget.Pause_MenuWidget_C"))
        (`UserWidget.AddToViewport` _returnvalue_2 0)
        (`GameplayStatics.SetGamePaused` true)
        (set `PlayerController.bShowMouseCursor` true _returnvalue))
      (:`B`
        (`Widget.RemoveFromParent` _returnvalue_2)
        (`GameplayStatics.SetGamePaused` false)
        (set `PlayerController.bShowMouseCursor` false _returnvalue)))))

(fn `UserConstructionScript`)