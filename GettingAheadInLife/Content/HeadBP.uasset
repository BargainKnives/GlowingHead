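; HeadBP is a player-controlled Head that rolls in response to movement input.
; The MoveForward and MoveRight axes apply torque around world Y and X respectively, each scaled by RollTorque and negated.
; Movement is physics-driven through torque on the Head component, with mass taken into account and no camera-relative steering.
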(event `InputAxis|MoveForward`
  (params (AxisValue :type "Float (single-precision)"))
  ;[1 0 0.01667 0.686] Move Forward & Backward
  (`PrimitiveComponent.AddTorqueInRadians` (`self.Head`) (`KismetMathLibrary.MakeVector` 0.0 (* (`self.RollTorque`) AxisValue -1.0)) "None" false))

(event `InputAxis|MoveRight`
  (params (AxisValue :type "Float (single-precision)"))
  ;[1 0 0.02469 0.686] Move Left & Right
  (`PrimitiveComponent.AddTorqueInRadians` (`self.Head`) (`KismetMathLibrary.MakeVector` (* (`self.RollTorque`) AxisValue -1.0)) "None" false))

(fn `UserConstructionScript`)